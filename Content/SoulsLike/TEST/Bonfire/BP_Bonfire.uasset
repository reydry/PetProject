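; BP_Bonfire is a souls-like bonfire that offers an interaction to the player character when nearby.
; It creates an interact widget at BeginPlay and shows or removes it as BP_SoulsCharacter enters or leaves its sphere.
; The same overlaps add and remove the IMC_Bonfire input mapping context, so bonfire input is scoped to proximity.
; UseBonfire broadcasts OnBonfireUsed and hides the prompt, and EndUsingBonfire shows it again.
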(event `self.ReceiveBeginPlay`
  (bind _returnvalue (`|CreateWidget` "/Game/SoulsLike/TEST/Bonfire/W_InteractWidget.W_InteractWidget_C"))
  (set `self.Widget` _returnvalue))

(event `self.Sphere.OnComponentBeginOverlap`
  (params (OverlappedComponent :type "PrimitiveComponent Object Reference") (OtherActor :type "Actor Object Reference") (OtherComp :type "PrimitiveComponent Object Reference") (OtherBodyIndex :type Integer) (bFromSweep :type Boolean) (SweepResult :type "HitResult Structure (by ref)"))
  (bind _asbp_souls_character (cast `/Game/SoulsLike/Character/BP_SoulsCharacter` OtherActor))
  (`/Game/SoulsLike/Character/BP_SoulsCharacter.AddInputMappingContext` _asbp_souls_character "/Game/SoulsLike/TEST/Bonfire/IMC_Bonfire.IMC_Bonfire")
  (`UserWidget.AddToViewport` (`self.Widget`) 0))

(event `self.Sphere.OnComponentEndOverlap`
  (params (OverlappedComponent :type "PrimitiveComponent Object Reference") (OtherActor :type "Actor Object Reference") (OtherComp :type "PrimitiveComponent Object Reference") (OtherBodyIndex :type Integer))
  (bind _asbp_souls_character (cast `/Game/SoulsLike/Character/BP_SoulsCharacter` OtherActor))
  (`/Game/SoulsLike/Character/BP_SoulsCharacter.RemoveInputMappingContext` _asbp_souls_character "/Game/SoulsLike/TEST/Bonfire/IMC_Bonfire.IMC_Bonfire")
  (`Widget.RemoveFromParent` (`self.Widget`)))

(event `UseBonfire`
  (`self.OnBonfireUsed`)
  (`Widget.RemoveFromParent` (`self.Widget`)))

(event `EndUsingBonfire`
  (`UserWidget.AddToViewport` (`self.Widget`) 0))

(fn `UserConstructionScript`)