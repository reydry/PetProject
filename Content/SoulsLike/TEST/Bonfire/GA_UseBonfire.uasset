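; Gameplay ability for resting at a souls-like bonfire and changing character stats, triggered by a gameplay event targeting a BP_Bonfire.
; On commit it starts bonfire use and shows W_BonfireMenu with current Vigor, Endurance and Mind in UI-only input.
; Applying writes the widget's tag-to-value map into GE_UpdateStats as SetByCaller magnitudes, then applies GE_PostInitAttributes.
; Ending the ability restores game input and ends bonfire use.
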(event `self.K2_ActivateAbilityFromEvent`
  (params (EventData :type "GameplayEventData Structure (by ref)"))
  (bind _returnvalue (`self.K2_CommitAbility`))
  (if _returnvalue
    (bind _asbp_bonfire (cast `/Game/SoulsLike/TEST/Bonfire/BP_Bonfire` (`.Target` (break `GameplayEventData` EventData))))
    (`/Game/SoulsLike/TEST/Bonfire/BP_Bonfire.UseBonfire` _asbp_bonfire)
    (`self.ShowBonfireMenu`)
    (else
      (`self.K2_EndAbility`))))

(event `self.K2_OnEndAbility`
  (params (bWasCancelled :type Boolean))
  (`self.HideBonfireMenu`)
  (bind _asbp_bonfire (cast `/Game/SoulsLike/TEST/Bonfire/BP_Bonfire` (`.Target` (break `GameplayEventData` (`self.CurrentEventData`)))))
  (`/Game/SoulsLike/TEST/Bonfire/BP_Bonfire.EndUsingBonfire` _asbp_bonfire))

(event `ApplyNewStats`
  (`self.ApplyStatChanges`))

(fn `ApplyStatChanges`
  (set `self.GamepleyEffectSpec` (`self.MakeOutgoingGameplayEffectSpec` "/Game/SoulsLike/TEST/Bonfire/GE_UpdateStats.GE_UpdateStats_C"))
  (bind _newstats (`/Game/SoulsLike/TEST/Bonfire/W_BonfireMenu.GetNewStats` (`self.BonfireWidget`)))
  (bind _keys (`BlueprintMapLibrary.Map_Keys` _newstats))
  (for _array_element _keys
    (`AbilitySystemBlueprintLibrary.AssignTagSetByCallerMagnitude` (`self.GamepleyEffectSpec`) _array_element (`KismetMathLibrary.Conv_IntToDouble` (`BlueprintMapLibrary.Map_Find` _newstats _array_element))))
  (`self.K2_ApplyGameplayEffectSpecToOwner` (`self.GamepleyEffectSpec`))
  (`self.BP_ApplyGameplayEffectToOwner` "/Game/SoulsLike/Stats/GE_PostInitAttributes.GE_PostInitAttributes_C"))

(fn `Get Player Controller`
  (returns (PlayerController :type "PlayerController Object Reference"))
  (bind _aspawn (cast `Pawn` (`self.GetAvatarActorFromActorInfo`)))
  (bind _asplayer_controller (cast `PlayerController` (`Pawn.GetController` _aspawn)))
  (return _asplayer_controller))

(fn `HideBonfireMenu`
  (bind _playercontroller (`self.Get Player Controller`))
  (`/Engine/EditorBlueprintResources/StandardMacros.IsValid` _playercontroller
    (:`Is Valid`
      (`WidgetBlueprintLibrary.SetInputMode_GameOnly` _playercontroller)
      (set `PlayerController.bShowMouseCursor` false _playercontroller))))

(fn `SetupStatsInWidget`
  (params (Menu :type "/Game/SoulsLike/TEST/Bonfire/W_BonfireMenu Object Reference"))
  (bind _returnvalue (`self.GetAbilitySystemComponentFromActorInfo`))
  (bind _map (`|MakeMap` "Vigor" (`.ReturnValue` (`AbilitySystemBlueprintLibrary.GetFloatAttributeFromAbilitySystemComponent` _returnvalue (struct :`AttributeName` "Vigor" :`Attribute` "/Script/PetProject.PPSoulsSet:Vigor" :`AttributeOwner` "/Script/CoreUObject.Class'/Script/PetProject.PPSoulsSet'"))) "Endurance" (`.ReturnValue` (`AbilitySystemBlueprintLibrary.GetFloatAttributeFromAbilitySystemComponent` _returnvalue (struct :`AttributeName` "Endurance" :`Attribute` "/Script/PetProject.PPSoulsSet:Endurance" :`AttributeOwner` "/Script/CoreUObject.Class'/Script/PetProject.PPSoulsSet'"))) "Mind" (`.ReturnValue` (`AbilitySystemBlueprintLibrary.GetFloatAttributeFromAbilitySystemComponent` _returnvalue (struct :`AttributeName` "Mind" :`Attribute` "/Script/PetProject.PPSoulsSet:Mind" :`AttributeOwner` "/Script/CoreUObject.Class'/Script/PetProject.PPSoulsSet'")))))
  (bind _keys (`BlueprintMapLibrary.Map_Keys` _map))
  (bind _outtextblocks (`/Game/SoulsLike/TEST/Bonfire/W_BonfireMenu.GetStatTextBlocks` Menu))
  (for _array_element _keys
    (set `TextBlock.Text` (`KismetTextLibrary.Conv_DoubleToText` (`BlueprintMapLibrary.Map_Find` _map _array_element) "HalfToEven") (`BlueprintMapLibrary.Map_Find` _outtextblocks _array_element))))

(fn `ShowBonfireMenu`
  (bind _returnvalue (`|CreateWidget` "/Game/SoulsLike/TEST/Bonfire/W_BonfireMenu.W_BonfireMenu_C"))
  (bind _output_get (set `self.BonfireWidget` _returnvalue))
  (`self.SetupStatsInWidget` _output_get)
  (`UserWidget.AddToViewport` _returnvalue 0)
  (`WidgetBlueprintLibrary.SetInputMode_UIOnlyEx` (`self.Get Player Controller`) (`self.BonfireWidget`))
  (set `PlayerController.bShowMouseCursor` true (`self.Get Player Controller`))
  (add `Button.OnClicked` (`/Game/SoulsLike/TEST/Bonfire/W_BonfireMenu.B_Leave` (`self.BonfireWidget`)) (`|CreateDelegate` :!event `K2_EndAbility`))
  (add `Button.OnClicked` (`/Game/SoulsLike/TEST/Bonfire/W_BonfireMenu.B_Apply` (`self.BonfireWidget`)) (`|CreateDelegate` :!event `ApplyNewStats`)))