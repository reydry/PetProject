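; Gameplay ability for drinking a potion, gated on the player controller's inventory holding at least one of the item.
; On activation it commits, starts the drink montage and immediately applies the potion's gameplay effect to the owner, without waiting for the animation.
; Only montage completion explicitly ends the ability; interruption is unhandled.
; OnEndAbility consumes one item from the inventory, however the ability ends.
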(event `self.K2_ActivateAbility`
  (`self.K2_CommitAbility`)
  (`AbilityTask_PlayMontageAndWait.CreatePlayMontageAndWaitProxy` "None" "/Game/SoulsLike/TEST/Anim/AM_Drink_Potion.AM_Drink_Potion"
    (:`then`
      (`self.BP_ApplyGameplayEffectToOwner` (`self.Effect`)))
    (:`OnCompleted`
      (`self.K2_EndAbility`))))

(event `self.K2_OnEndAbility`
  (params (bWasCancelled :type Boolean))
  (`PPInventoryComponent.ConsumeItem` (`self.GetInventory`) (`self.Item`) 1 true))

(fn `GetInventory`
  (returns (inventory :type "PPInventoryComponent Object Reference"))
  (bind (_returnvalue_owneractor _returnvalue_avataractor _returnvalue_playercontroller) (break `GameplayAbilityActorInfo` (`self.GetActorInfo`)))
  (return (`PPInventoryComponent.GetInventoryComponentFromActor` _returnvalue_playercontroller)))

(fn `K2_CanActivateAbility`
  (params (ActorInfo :type "GameplayAbilityActorInfo Structure") (Handle :type "GameplayAbilitySpecHandle Structure"))
  (returns (RelevantTags :type "GameplayTagContainer Structure") (ReturnValue :type Boolean))
  (bind (_returnvalue_itemtype _returnvalue_itemcount) (break `PPItemData` (`PPInventoryComponent.GetItemData` (`PPInventoryComponent.GetInventoryComponentFromActor` ActorInfo_PlayerController) (`self.Item`))))
  (return (struct) (> _returnvalue_itemcount 0)))