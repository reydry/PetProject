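; Base melee weapon Gameplay Ability for the SoulsLike game, providing helper functions for hit detection and damage.
; TracingObjects sphere-traces Pawns between the weapon mesh's bottom and top sockets, ignoring the avatar, with debug drawing enabled.
; Hit actors on a different PlayerState team are stored uniquely, and OnTargetDataReady applies DamageEffect to each.
; The event graph is empty, so nothing here triggers tracing, damage or array clearing.
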(fn `ClearTargetArray`
  (`KismetArrayLibrary.Array_Clear` (`self.TargetsArray`)))

(fn `GetActorsToIgnore`
  (returns (ActorsToIgnore :type "Array of Actor Object Reference"))
  (return (`|MakeArray` (`self.GetAvatarActorFromActorInfo`))))

(fn `GetObjectTypes`
  (returns (ObjectTypes :type "Array of EObjectTypeQuery Enum"))
  (return (`|MakeArray` "ObjectTypeQuery3" :!type "EObjectTypeQuery Enum")))

(fn `IsTargetInEnemyTeam`
  (params (Target :type "Actor Object Reference"))
  (returns (IsEnemy :type Boolean))
  (bind _returnvalue_owneractor (break `GameplayAbilityActorInfo` (`self.GetActorInfo`)))
  (`/Engine/EditorBlueprintResources/StandardMacros.IsValid` Target
    (:`Is Valid`
      (bind _playerstate (message `/Game/SoulsLike/BPIterfaces/BPI_Character.GetPPPlayerState` _returnvalue_owneractor))
      (bind _playerstate_2 (message `/Game/SoulsLike/BPIterfaces/BPI_Character.GetPPPlayerState` (`local.Target`)))
      (return (`|EnumInequality` (`PPPlayerState.Team` _playerstate) (`PPPlayerState.Team` _playerstate_2))))))

(fn `OnTargetDataReady`
  (for _array_element (`self.TargetsArray`)
    (`self.BP_ApplyGameplayEffectToTarget` (`AbilitySystemBlueprintLibrary.AbilityTargetDataFromActor` _array_element) (`self.DamageEffect`))))

(fn `TracingObjects`
  (bind _returnvalue (`PPBaseWeapon.GetMesh` (`self.Weapon`)))
  (bind _outhit (`KismetSystemLibrary.SphereTraceSingleForObjects` (`SceneComponent.GetSocketLocation` _returnvalue "BottomSocket") (`SceneComponent.GetSocketLocation` _returnvalue "TopSocket") 50.0 (`self.GetObjectTypes`) false (`self.GetActorsToIgnore`) "ForDuration" true (struct :`R` 1.0 :`A` 1.0) (struct :`G` 1.0 :`A` 1.0) 0.1))
  (bind (_bblockinghit _binitialoverlap _time _distance _location _impactpoint _normal _impactnormal _physmat _hitactor) (`GameplayStatics.BreakHitResult` _outhit))
  (if (`self.IsTargetInEnemyTeam` _hitactor)
    (`KismetArrayLibrary.Array_AddUnique` (`self.TargetsArray`) _hitactor)))