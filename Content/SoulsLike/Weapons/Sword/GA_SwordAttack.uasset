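; Gameplay Ability for a Souls-like sword attack that commits, fetches the avatar's current weapon and plays its current combo montage.
; Gameplay events during the montage trigger object tracing and target-data handling, using functions defined outside this graph.
; It clears targets at activation and blocks stamina regeneration with a loose tag, removed when the ability ends.
; The ability ends when the montage completes, blends out, is interrupted or is cancelled, or if commit fails.
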(event `self.K2_ActivateAbility`
  (bind _returnvalue (`self.K2_CommitAbility`))
  (if _returnvalue
    (`self.SetWeapon`)
    (`AbilityTask_PlayMontageAndWait.CreatePlayMontageAndWaitProxy` "None" (`self.GetMontage`)
      (:`then`
        (`AbilityTask_WaitGameplayEvent.WaitGameplayEvent` (struct :`TagName` "GameplayEvent.TraceObjects") null
          (:`then`
            (`AbilityTask_WaitGameplayEvent.WaitGameplayEvent` (struct :`TagName` "GameplayEvent.TargetDataReady") null
              (:`then`
                (`self.ClearTargetArray`)
                (`AbilitySystemBlueprintLibrary.AddLooseGameplayTags` (`self.GetAvatarActorFromActorInfo`) (`BlueprintGameplayTagLibrary.MakeGameplayTagContainerFromTag` (struct :`TagName` "Attribute.Stamina.CannotRegenerate"))))
              (:`EventReceived`
                (`self.OnTargetDataReady`))))
          (:`EventReceived`
            (`self.TracingObjects`))))
      (:`OnCompleted`
        (`self.K2_EndAbility` :!label _label))
      (:`OnBlendOut`
        (goto _label))
      (:`OnInterrupted`
        (goto _label))
      (:`OnCancelled`
        (goto _label)))
    (else
      (`self.K2_EndAbility`))))

(event `self.K2_OnEndAbility`
  (params (bWasCancelled :type Boolean))
  (`AbilitySystemBlueprintLibrary.RemoveLooseGameplayTags` (`self.GetAvatarActorFromActorInfo`) (`BlueprintGameplayTagLibrary.MakeGameplayTagContainerFromTag` (struct :`TagName` "Attribute.Stamina.CannotRegenerate"))))

(fn `GetMontage`
  (returns (Montage :type "AnimMontage Object Reference"))
  (bind _newparam (message `/Game/SoulsLike/BPIterfaces/BPI_Inventory.GetCurrentComboMontage` (`self.GetAvatarActorFromActorInfo`)))
  (return _newparam))

(fn `SetWeapon`
  (bind _currentweapon (message `/Game/SoulsLike/BPIterfaces/BPI_Inventory.GetCurrentWeaponObject` (`self.GetAvatarActorFromActorInfo`)))
  (set `self.Weapon` _currentweapon))