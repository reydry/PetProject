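; Base melee attack gameplay ability that plays a combo attack montage and applies damage to the targets it hits.
; On activation it commits, then plays one of four slow primary-attack montages selected by the avatar's current combo montage index.
; While the montage runs, it waits for a TargetDataReady gameplay event and applies DamageEffect to that event's target data.
; The ability ends when the montage completes, blends out, is interrupted or cancelled, or when commit fails.
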(event `self.K2_ActivateAbility`
  (bind _returnvalue (`self.K2_CommitAbility`))
  (if _returnvalue
    (`AbilityTask_PlayMontageAndWait.CreatePlayMontageAndWaitProxy` "None" (`self.GetMontage`)
      (:`then`
        (bind (_asynctaskproxy _payload) (`AbilityTask_WaitGameplayEvent.WaitGameplayEvent` (struct :`TagName` "GameplayEvent.TargetDataReady") null)
          (:`EventReceived`
            (`self.BP_ApplyGameplayEffectToTarget` (`.TargetData` (break `GameplayEventData` _payload)) (`self.DamageEffect`)))))
      (:`OnCompleted`
        (`self.K2_EndAbility` :!label _label))
      (:`OnBlendOut`
        (goto _label))
      (:`OnInterrupted`
        (goto _label))
      (:`OnCancelled`
        (goto _label)))
    (else
      (`self.K2_EndAbility`))))

(fn `GetMontage`
  (returns (Montage :type "AnimMontage Object Reference"))
  (bind _combo (message `/Game/SoulsLike/BPIterfaces/BPI_Character.GetCurrentComboMontage` (`self.GetAvatarActorFromActorInfo`)))
  (return (select `int` _combo :`0` "/Game/SoulsLike/Character/Animations/PrimaryAttack_A_Slow_Montage.PrimaryAttack_A_Slow_Montage" :`1` "/Game/SoulsLike/Character/Animations/PrimaryAttack_B_Slow_Montage.PrimaryAttack_B_Slow_Montage" :`2` "/Game/SoulsLike/Character/Animations/PrimaryAttack_C_Slow_Montage.PrimaryAttack_C_Slow_Montage" :`3` "/Game/SoulsLike/Character/Animations/PrimaryAttack_D_Slow_Montage.PrimaryAttack_D_Slow_Montage" :!type "AnimMontage Object Reference")))