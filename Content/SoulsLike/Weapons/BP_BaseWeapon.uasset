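; BP_BaseWeapon is the base weapon actor that reports melee overlap hits on enemy targets through the Gameplay Ability System.
; Gameplay events on its instigator toggle the collision component between query-only and disabled.
; Overlaps check that both actors' player states have differing teams, then send a TargetDataReady event carrying the hit actor as target data back to the instigator.
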(event `self.ReceiveBeginPlay`
  (`AbilityAsync_WaitGameplayEvent.WaitGameplayEventToActor` (`self.GetInstigator`) (struct :`TagName` "GameplayEvent.Collision.Enable")
    (:`then`
      (`AbilityAsync_WaitGameplayEvent.WaitGameplayEventToActor` (`self.GetInstigator`) (struct :`TagName` "GameplayEvent.Collision.Disable")
        (:`EventReceived`
          (`self.DisableCollision`))))
    (:`EventReceived`
      (`self.EnableCollision`))))

(event `self.Collision.OnComponentBeginOverlap`
  (params (OverlappedComponent :type "PrimitiveComponent Object Reference") (OtherActor :type "Actor Object Reference") (OtherComp :type "PrimitiveComponent Object Reference") (OtherBodyIndex :type Integer) (bFromSweep :type Boolean) (SweepResult :type "HitResult Structure (by ref)"))
  (bind _returnvalue (`self.GetInstigator`))
  (if (`self.IsTargetInEnemyTeam` OtherActor _returnvalue)
    (`AbilitySystemBlueprintLibrary.SendGameplayEventToActor` _returnvalue (struct :`TagName` "GameplayEvent.TargetDataReady") (make `GameplayEventData` (struct :`TagName` "GameplayEvent.TargetDataReady") null null null null (struct) (struct) (struct) 0.0 (`AbilitySystemBlueprintLibrary.AbilityTargetDataFromActor` OtherActor)))))

(fn `DisableCollision`
  (`PrimitiveComponent.SetCollisionEnabled` (`self.Collision`) "NoCollision"))

(fn `EnableCollision`
  (`PrimitiveComponent.SetCollisionEnabled` (`self.Collision`) "QueryOnly"))

(fn `IsTargetInEnemyTeam`
  (params (Target :type "Actor Object Reference") (WeaponOwner :type "Actor Object Reference"))
  (returns (IsEnemy :type Boolean))
  (bind _playerstate (message `/Game/SoulsLike/BPIterfaces/BPI_Character.GetPPPlayerState` Target))
  (bind _playerstate_2 (message `/Game/SoulsLike/BPIterfaces/BPI_Character.GetPPPlayerState` WeaponOwner))
  (if (and (`KismetSystemLibrary.IsValid` _playerstate) (`KismetSystemLibrary.IsValid` _playerstate_2))
    (return (`|EnumInequality` (`PPPlayerState.Team` _playerstate_2) (`PPPlayerState.Team` _playerstate)))
    (else
      (return false))))

(fn `UserConstructionScript`)