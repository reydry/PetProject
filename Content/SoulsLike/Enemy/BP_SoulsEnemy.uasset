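; Souls-like enemy character that wields a sword and displays its health through a widget.
; On BeginPlay it spawns BP_Sword into the hand socket, applies an attribute-initializing GameplayEffect through GAS and binds to health component attribute changes.
; Each change updates the W_EnemyHealth ratio, with a DoOnce making the bar visible the first time.
; Getter functions supply the current weapon and a fixed slow primary-attack combo montage.
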(event `self.ReceiveBeginPlay`
  (bind _returnvalue (`AbilitySystemBlueprintLibrary.GetAbilitySystemComponent` null))
  (bind _returnvalue_2 (`|SpawnActorFromClass` "/Game/SoulsLike/Weapons/Sword/BP_Sword.BP_Sword_C" (`self.GetTransform`) "Undefined" "MultiplyWithRoot" null null))
  (bind _output_get (set `self.CurrentWeapon` _returnvalue_2))
  (`self.K2_AttachToComponent` _output_get (`self.Mesh`) "HandSocket" "SnapToTarget" "SnapToTarget" "SnapToTarget" true)
  (`/Engine/EditorBlueprintResources/StandardMacros.IsValid` _returnvalue
    (:`Is Valid`
      (`AbilitySystemComponent.BP_ApplyGameplayEffectToSelf` :`self` _returnvalue :`GameplayEffectClass` "/Game/SoulsLike/Stats/GE_PostInitAttributes.GE_PostInitAttributes_C")
      (add `PPHealthComponent.OnAttributeChangedDelegateHandle` (`PPHealthComponent.GetHealthComponentFromActor` self) (`|CreateDelegate` :!event `OnAttributeChangedDelegateHandle_Event`)))))

(event `OnAttributeChangedDelegateHandle_Event`
  (params (NewValue :type "Float (single-precision)") (MaxValue :type "Float (single-precision)") (AttributeName :type String))
  (bind _asw_enemy_health (cast `/Game/SoulsLike/UI/W_EnemyHealth` (`WidgetComponent.GetUserWidgetObject` (`self.Health`))))
  (`/Game/SoulsLike/UI/W_EnemyHealth.SetHealth` _asw_enemy_health (/ NewValue MaxValue))
  (`/Engine/EditorBlueprintResources/StandardMacros.DoOnce` false
    (:`Completed`
      (`Widget.SetVisibility` _asw_enemy_health "Visible"))))

(fn `GetCurrentComboMontage`
  (returns (NewParam :type "AnimMontage Object Reference"))
  (return "/Game/SoulsLike/Character/Animations/PrimaryAttack_A_Slow_Montage.PrimaryAttack_A_Slow_Montage"))

(fn `GetCurrentWeaponObject`
  (returns (CurrentWeapon :type "PPBaseWeapon Object Reference"))
  (return (`self.CurrentWeapon`)))

(fn `UserConstructionScript`)