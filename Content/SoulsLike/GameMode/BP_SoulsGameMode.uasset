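; Souls-like game mode that runs numbered enemy waves and handles game over.
; Each wave reads its enemy classes, counts, levels and duration from the Wave data table, spawning at randomly offset BP_EnemySpawner locations.
; The next wave starts when all spawned enemies are destroyed or a one-second looping countdown expires, showing a wave widget.
; Player character destruction shows the game-over widget and cursor and stops the countdown.
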(event `self.ReceiveBeginPlay`
  (`self.SetupSpawners`)
  (`self.SetupEvents`)
  (`self.SpawnWave`))

(event `SetupSpawners`
  (bind _outactors (`GameplayStatics.GetAllActorsOfClass` "/Game/SoulsLike/Spawner/BP_EnemySpawner.BP_EnemySpawner_C"))
  (set `self.Spawners` _outactors)
  (set `self.WaveNum` 0))

(event `RespawnWave`
  (if (== (`self.SpawnedEnemies`) 0)
    (`self.SpawnWave`)))

(event `SpawnWave`
  (`self.ClearTimer`)
  (`/Engine/EditorBlueprintResources/StandardMacros.IncrementInt` (`self.WaveNum`)
    (:`  `
      (`self.SpawnEnemies`)
      (`self.ShowWaveUI`)
      (`self.SetupTimer`))))

(event `OnEnemyDestroy` :!signature `self.OnDestroyed`
  (params (DestroyedPawn :type "Actor Object Reference"))
  (remove `self.OnDestroyed` DestroyedPawn (`|CreateDelegate` :!event `OnEnemyDestroy`))
  (`/Engine/EditorBlueprintResources/StandardMacros.DecrementInt` (`self.SpawnedEnemies`)
    (:`  `
      (`self.RespawnWave`))))

(event `TimeElapsed`
  (bind _result (`/Engine/EditorBlueprintResources/StandardMacros.DecrementInt` (`self.WaveRespawnTime`))
    (:`  `
      (if (== _result 0)
        (`self.SpawnWave`)))))

(event `SetupTimer`
  ;[1 1 1] Comment
  (bind _returnvalue (`KismetSystemLibrary.K2_SetTimerDelegate` (`|CreateDelegate` :!event `TimeElapsed`) 1.0 true))
  (set `self.RespawnTimer` _returnvalue))

(event `ClearTimer`
  ;[1 1 1] Comment
  (`KismetSystemLibrary.K2_ClearAndInvalidateTimerHandle` (`self.RespawnTimer`)))

(fn `ClearEvents`
  (remove `self.OnDestroyed` (`GameplayStatics.GetPlayerCharacter` 0) (`|CreateDelegate` :!event `OnCharacterDeath`))
  (`KismetSystemLibrary.K2_ClearAndInvalidateTimerHandle` (`self.RespawnTimer`)))

(fn `GameOver`
  (bind _returnvalue (`|CreateWidget` "/Game/SoulsLike/UI/GameOver/W_GameOver.W_GameOver_C"))
  (`UserWidget.AddToViewport` _returnvalue 0))

(fn `GetSpawnPoint`
  (returns (SpawnPoint :type "Transform Structure"))
  (bind _returnvalue (`KismetMathLibrary.RandomFloatInRange` -200.0 200.0))
  (bind _spawners (`self.Spawners`))
  (bind _returnvalue_2 (`self.GetTransform` (`|GetArrayItem` _spawners (`KismetMathLibrary.RandomIntegerInRange` 0 (`KismetArrayLibrary.Array_LastIndex` _spawners)))))
  (return (`KismetMathLibrary.MakeTransform` (`KismetMathLibrary.MakeVector` (+ _returnvalue (.x (.location _returnvalue_2))) (+ _returnvalue (.y (.location _returnvalue_2))) (+ (.z (.location _returnvalue_2)) _returnvalue)) (.rotation _returnvalue_2) (.scale _returnvalue_2))))

(fn `OnCharacterDeath`
  (params (Character :type "Actor Object Reference"))
  (`self.GameOver`)
  (set `PlayerController.bShowMouseCursor` true (`GameplayStatics.GetPlayerController` 0))
  (`self.ClearEvents`))

(fn `SetupEvents`
  (add `self.OnDestroyed` (`GameplayStatics.GetPlayerCharacter` 0) (`|CreateDelegate` :!event `OnCharacterDeath`)))

(fn `ShowWaveUI`
  (bind _returnvalue (`|CreateWidget` "/Game/SoulsLike/UI/Wave/W_Wave.W_Wave_C"))
  (set `/Game/SoulsLike/UI/Wave/W_Wave.WaveNum` (`KismetStringLibrary.Conv_IntToString` (`self.WaveNum`)) _returnvalue)
  (`UserWidget.AddToViewport` _returnvalue 0))

(fn `SpawnEnemies`
  (bind _returnvalue (`|GetDataTableRow` "/Game/SoulsLike/Wave/Wave.Wave" (`KismetStringLibrary.Conv_StringToName` (`KismetStringLibrary.Concat_StrStr` "Wave_" (`KismetStringLibrary.Conv_IntToString` (`self.WaveNum`)))))
    (:`then`
      (bind (_enemies _wavetime) (break `/Game/SoulsLike/Wave/WavesStruct` _returnvalue))
      (set `self.WaveRespawnTime` _wavetime)
      (for _array_element _enemies
        (bind (_enemy _level _count) (break `/Game/SoulsLike/Wave/EnemiesStruct` _array_element))
        (for _ (range 1 (+ _count 1))
          (bind _returnvalue_2 (`|SpawnActorFromClass` _enemy (`self.GetSpawnPoint`) "AdjustIfPossibleButAlwaysSpawn" "MultiplyWithRoot" null _level null))
          (add `self.OnDestroyed` _returnvalue_2 (`|CreateDelegate` :!event `OnEnemyDestroy`))
          (`/Engine/EditorBlueprintResources/StandardMacros.IncrementInt` (`self.SpawnedEnemies`)))))))

(fn `UserConstructionScript`)