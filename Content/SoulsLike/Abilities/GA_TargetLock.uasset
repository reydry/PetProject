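; Gameplay ability that locks the souls-like character's camera onto a target pawn.
; On activation it sphere-traces along the camera's forward vector from the character's location, ignoring itself, and takes the first hit as the target.
; A valid target is passed to the character's PPCameraLockComponent, which stays locked until a TargetLost gameplay event ends the ability.
; Ending the ability clears the target and releases the lock.
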(event `self.K2_ActivateAbility`
  (bind _returnvalue (`self.K2_CommitAbility`))
  (if _returnvalue
    (`self.InitAbilityData`)
    (`self.FindTarget`)
    (if (`self.IsLockDataValid`)
      (`self.SetLockData` true)
      (`AbilityTask_WaitGameplayEvent.WaitGameplayEvent` (struct :`TagName` "GameplayEvent.TargetLost") null
        (:`EventReceived`
          (`KismetSystemLibrary.PrintString` "target lost")
          (`self.K2_EndAbility`)))
      (else
        (`self.K2_EndAbility`)))
    (else
      (`self.K2_EndAbility`))))

(event `self.K2_OnEndAbility`
  (params (bWasCancelled :type Boolean))
  (set `self.Target` null)
  (`self.SetLockData` false))

(fn `FindTarget`
  (bind _location (`self.Location`))
  (bind _outhit (`KismetSystemLibrary.SphereTraceSingleForObjects` _location (+ _location (* (`self.ForwardVector`) 650.0)) 100.0 (`self.GetObjectType`) false (`self.GetActorsToIgnore`)))
  (set `self.Target` (`.HitActor` (`GameplayStatics.BreakHitResult` _outhit))))

(fn `GetActorsToIgnore`
  (returns (ActorsToIgnore :type "Array of Actor Object Reference"))
  (return (`|MakeArray` (`self.GetAvatarActorFromActorInfo`))))

(fn `GetObjectType`
  (returns (ObjectType :type "Array of EObjectTypeQuery Enum"))
  (return (`|MakeArray` "ObjectTypeQuery3" :!type "EObjectTypeQuery Enum")))

(fn `InitAbilityData`
  (bind _asbp_souls_character (cast `/Game/SoulsLike/Character/BP_SoulsCharacter` (`self.GetAvatarActorFromActorInfo`)))
  (set `self.Location` (`Actor.K2_GetActorLocation` _asbp_souls_character))
  (set `self.ForwardVector` (`SceneComponent.GetForwardVector` (`/Game/SoulsLike/Character/BP_SoulsCharacter.Camera` _asbp_souls_character)))
  (set `self.CameraLockComponent` (`Actor.GetComponentByClass` _asbp_souls_character "/Script/PetProject.PPCameraLockComponent")))

(fn `IsLockDataValid`
  (returns (IsDataValid :type Boolean))
  (return (and (`KismetSystemLibrary.IsValid` (`self.Target`)) (`KismetSystemLibrary.IsValid` (`self.CameraLockComponent`)))))

(fn `SetLockData`
  (params (bLockOnTarget :type Boolean))
  (bind _cameralockcomponent (`self.CameraLockComponent`))
  (`PPCameraLockComponent.SetTarget` _cameralockcomponent (`self.Target`))
  (`PPCameraLockComponent.SetLockOnTarget` _cameralockcomponent bLockOnTarget))