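; Gameplay ability that switches the player's camera lock-on to another enemy, using the event magnitude's sign as direction.
; It fans sphere traces from camera forward toward that side, ignoring the avatar and current target, collecting BP_TestSoulsEnemy hits.
; GetClosestEnemy's result goes to PPCameraLockComponent, though its distance loop assigns the avatar, not the nearer enemy, when one is found.
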(event `self.K2_ActivateAbilityFromEvent`
  (params (EventData :type "GameplayEventData Structure (by ref)"))
  (bind _returnvalue (`self.K2_CommitAbility`))
  (if _returnvalue
    (`self.InitTraceData`)
    (bind _closestenemy (`self.GetClosestEnemy` (`.EventMagnitude` (break `GameplayEventData` EventData))))
    (`/Engine/EditorBlueprintResources/StandardMacros.IsValid` _closestenemy
      (:`Is Valid`
        (`PPCameraLockComponent.SetTarget` (`Actor.GetComponentByClass` (`self.GetAvatarActorFromActorInfo`) "/Script/PetProject.PPCameraLockComponent") _closestenemy))
      (:`Is Not Valid`
        _))
    (`self.K2_EndAbility`)
    (else
      (`self.K2_EndAbility`))))

(fn `FindTargets`
  (params (InDirection :type "Float (double-precision)"))
  (bind _startlocation (`self.StartLocation`))
  (`KismetArrayLibrary.Array_Clear` (`self.HitResults`))
  (if (< InDirection 0.0)
    (set `self.Angle` -15.0)
    (else
      (set `self.Angle` 15.0)))
  (for _index (range 5)
    (bind _outhit (`KismetSystemLibrary.SphereTraceSingleForObjects` _startlocation (+ _startlocation (* (`KismetMathLibrary.RotateAngleAxis` (`self.ForwardVector`) (* _index (`self.Angle`)) (0.0 0.0 1.0)) 650.0)) 100.0 (`self.GetObjectType`) false (`self.GetActorsToIgnore`) "ForDuration" true (struct :`R` 1.0 :`A` 1.0) (struct :`G` 1.0 :`A` 1.0) 2.0))
    (bind (_bblockinghit _binitialoverlap _time _distance _location _impactpoint _normal _impactnormal _physmat _hitactor) (`GameplayStatics.BreakHitResult` _outhit))
    (cast `/Game/SoulsLike/TEST/BP_TestSoulsEnemy` _hitactor)
    (`KismetArrayLibrary.Array_AddUnique` (`self.HitResults`) _hitactor)))

(fn `GetActorsToIgnore`
  (returns (ActorsToIgnore :type "Array of Actor Object Reference"))
  (bind _returnvalue (`self.GetAvatarActorFromActorInfo`))
  (return (`|MakeArray` (`PPCameraLockComponent.GetTarget` (`Actor.GetComponentByClass` _returnvalue "/Script/PetProject.PPCameraLockComponent")) _returnvalue)))

(fn `GetClosestEnemy`
  (params (InDirection :type "Float (double-precision)"))
  (returns (ClosestEnemy :type "Actor Object Reference"))
  (bind _returnvalue (`self.GetAvatarActorFromActorInfo`))
  (`self.FindTargets` InDirection)
  (if (`KismetArrayLibrary.Array_IsValidIndex` (`self.HitResults`))
    (set `self.ClosestEnemy` (`|GetArrayItem` (`self.HitResults`)))
    (for _array_element (`self.HitResults`)
      (if (< (`Actor.GetDistanceTo` _array_element _returnvalue) (`Actor.GetDistanceTo` (`self.ClosestEnemy`) (`self.GetAvatarActorFromActorInfo`)))
        (set `self.ClosestEnemy` _returnvalue)))
    (return (`self.ClosestEnemy`))
    (else
      (return null))))

(fn `GetObjectType`
  (returns (NewParam :type "Array of EObjectTypeQuery Enum"))
  (return (`|MakeArray` "ObjectTypeQuery3" :!type "EObjectTypeQuery Enum")))

(fn `InitTraceData`
  (bind _asbp_souls_character (cast `/Game/SoulsLike/Character/BP_SoulsCharacter` (`self.GetAvatarActorFromActorInfo`)))
  (set `self.StartLocation` (`Actor.K2_GetActorLocation` _asbp_souls_character))
  (set `self.ForwardVector` (`SceneComponent.GetForwardVector` (`/Game/SoulsLike/Character/BP_SoulsCharacter.Camera` _asbp_souls_character))))