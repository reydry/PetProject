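; Gameplay ability for running in the SoulsLike game that raises the avatar character's walk speed while it is active.
; On activation it saves the character movement's MaxWalkSpeed in OldSpeed and applies a multiplier to it.
; When the ability ends it restores the saved speed.
; The graph never commits or ends the ability itself.
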(event `self.K2_ActivateAbility`
  (bind _ascharacter (cast `Character` (`self.GetAvatarActorFromActorInfo`)))
  (bind _charactermovement (`Character.CharacterMovement` _ascharacter))
  (bind _output_get (set `self.OldSpeed` (`CharacterMovementComponent.MaxWalkSpeed` _charactermovement)))
  (set `CharacterMovementComponent.MaxWalkSpeed` (* _output_get 1.5) _charactermovement))

(event `self.K2_OnEndAbility`
  (params (bWasCancelled :type Boolean))
  (bind _ascharacter (cast `Character` (`self.GetAvatarActorFromActorInfo`)))
  (set `CharacterMovementComponent.MaxWalkSpeed` (`self.OldSpeed`) (`Character.CharacterMovement` _ascharacter)))