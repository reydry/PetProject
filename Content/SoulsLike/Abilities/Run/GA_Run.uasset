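; Gameplay Ability for running in the SoulsLike game, raising the owner's walk speed by half while active.
; Activation requires a watched attribute above a small threshold, then saves and scales MaxWalkSpeed and applies the GA_RunCost effect.
; An attribute-change wait ends the ability when the value drops below that threshold.
; Ending restores the saved speed and removes the cost effect by its handle.
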(event `self.K2_ActivateAbility`
  (bind (_returnvalue_owneractor _returnvalue_avataractor _returnvalue_playercontroller _returnvalue_abilitysystemcomponent _returnvalue_skeletalmeshcomponent _returnvalue_animinstance _returnvalue_movementcomponent) (break `GameplayAbilityActorInfo` (`self.GetActorInfo`)))
  (`self.K2_CommitAbility`)
  (bind _ascharacter_movement_component (cast `CharacterMovementComponent` _returnvalue_movementcomponent))
  (`self.SetNewMoveSpeed` _ascharacter_movement_component)
  (`AbilityTask_WaitAttributeChange.WaitForAttributeChangeWithComparison` (struct :`AttributeName` "Stamina" :`Attribute` "/Script/PetProject.PPCharacterSet:Stamina" :`AttributeOwner` "/Script/CoreUObject.Class'/Script/PetProject.PPCharacterSet'") (struct) (struct) "LessThan" 2.0 true null
    (:`then`
      (bind _returnvalue (`self.BP_ApplyGameplayEffectToOwner` "/Game/SoulsLike/Abilities/Run/GA_RunCost.GA_RunCost_C"))
      (set `self.SpecHandle` _returnvalue))
    (:`OnChange`
      (`self.K2_EndAbility`))))

(event `self.K2_OnEndAbility`
  (params (bWasCancelled :type Boolean))
  (bind (_returnvalue_owneractor _returnvalue_avataractor _returnvalue_playercontroller _returnvalue_abilitysystemcomponent _returnvalue_skeletalmeshcomponent _returnvalue_animinstance _returnvalue_movementcomponent) (break `GameplayAbilityActorInfo` (`self.GetActorInfo`)))
  (bind _ascharacter_movement_component (cast `CharacterMovementComponent` _returnvalue_movementcomponent))
  (`self.SetOldMoveSpeed` _ascharacter_movement_component)
  (`self.BP_RemoveGameplayEffectFromOwnerWithHandle` (`self.SpecHandle`)))

(fn `K2_CanActivateAbility`
  (params (ActorInfo :type "GameplayAbilityActorInfo Structure") (Handle :type "GameplayAbilitySpecHandle Structure"))
  (returns (RelevantTags :type "GameplayTagContainer Structure") (ReturnValue :type Boolean))
  (return (struct) (> (`.ReturnValue` (`AbilitySystemBlueprintLibrary.GetFloatAttributeFromAbilitySystemComponent` (`.AbilitySystemComponent` (break `GameplayAbilityActorInfo` ActorInfo)) (struct :`AttributeName` "Stamina" :`Attribute` "/Script/PetProject.PPCharacterSet:Stamina" :`AttributeOwner` "/Script/CoreUObject.Class'/Script/PetProject.PPCharacterSet'"))) 2.0)))

(fn `SetNewMoveSpeed`
  (params (MovementComponent :type "CharacterMovementComponent Object Reference"))
  (bind _output_get (set `self.OldSpeed` (`CharacterMovementComponent.MaxWalkSpeed` MovementComponent)))
  (set `CharacterMovementComponent.MaxWalkSpeed` (* _output_get 1.5) (`local.MovementComponent`)))

(fn `SetOldMoveSpeed`
  (params (MovementComponent :type "CharacterMovementComponent Object Reference"))
  (set `CharacterMovementComponent.MaxWalkSpeed` (`self.OldSpeed`) MovementComponent))