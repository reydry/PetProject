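; Anim notify state that marks the trace window of an animation for the owning actor's Gameplay Ability System.
; Each tick it sends a GameplayEvent.TraceObjects event to the mesh owner, and on end it sends GameplayEvent.TargetDataReady.
; Both events fire only when the owner has a valid Ability System Component, and the notify does no tracing itself, leaving that to whatever handles the events.
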(fn `Received_NotifyEnd`
  (params (MeshComp :type "SkeletalMeshComponent Object Reference") (Animation :type "AnimSequenceBase Object Reference") (EventReference :type "AnimNotifyEventReference Structure (by ref)"))
  (returns (ReturnValue :type Boolean))
  (bind _returnvalue (`ActorComponent.GetOwner` MeshComp))
  (`/Engine/EditorBlueprintResources/StandardMacros.IsValid` (`AbilitySystemBlueprintLibrary.GetAbilitySystemComponent` _returnvalue)
    (:`Is Valid`
      (`AbilitySystemBlueprintLibrary.SendGameplayEventToActor` _returnvalue (struct :`TagName` "GameplayEvent.TargetDataReady") (make `GameplayEventData` (struct :`TagName` "GameplayEvent.TargetDataReady")))
      (return false))))

(fn `Received_NotifyTick`
  (params (MeshComp :type "SkeletalMeshComponent Object Reference") (Animation :type "AnimSequenceBase Object Reference") (FrameDeltaTime :type "Float (single-precision)") (EventReference :type "AnimNotifyEventReference Structure (by ref)"))
  (returns (ReturnValue :type Boolean))
  (bind _returnvalue (`ActorComponent.GetOwner` MeshComp))
  (`/Engine/EditorBlueprintResources/StandardMacros.IsValid` (`AbilitySystemBlueprintLibrary.GetAbilitySystemComponent` _returnvalue)
    (:`Is Valid`
      (`AbilitySystemBlueprintLibrary.SendGameplayEventToActor` _returnvalue (struct :`TagName` "GameplayEvent.TraceObjects") (make `GameplayEventData` (struct :`TagName` "GameplayEvent.TraceObjects")))
      (return false))))