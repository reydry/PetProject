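; Player controller for the Souls-like game that owns the HUD, pause menu and level-up buff selection.
; On possession it binds inventory and level-up delegates, creates or reveals the HUD, and forwards item changes to its icons; unpossessing hides it.
; Level-up pauses the game and opens a buff widget; the chosen HP, MP or SP bonus is applied with a matching restore through GAS effects, then pause toggles back.
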(event `self.ReceivePossess`
  (params (PossessedPawn :type "Pawn Object Reference"))
  (`self.SetupEvents` PossessedPawn)
  (`self.ShowHUD`)
  (message `/Game/SoulsLike/BPIterfaces/BPI_Character.SetupPlayer` PossessedPawn self))

(event `self.ReceiveUnPossess`
  (params (UnpossessedPawn :type "Pawn Object Reference"))
  (`self.ClearEvents` UnpossessedPawn)
  (`self.HideHUD`))

(event `/Game/SoulsLike/BPIterfaces/BPI_Controller.UpdateUI`
  (params (Item :type "PPItem Object Reference") (Slot :type "PPItemSlot Structure"))
  (message `/Game/SoulsLike/BPIterfaces/BPI_HUD.UpdateIcons` (`self.HUD`) Item (`PPInventoryComponent.GetItemData` (`self.BP_InventoryComponent`) Item)))

(event `OnInventoryItemChangedDelegateHandle_Event`
  (params (Item :type "PPItem Object Reference") (ItemData :type "PPItemData Structure"))
  (message `/Game/SoulsLike/BPIterfaces/BPI_HUD.UpdateIcons` (`self.HUD`) Item ItemData))

(event `/Game/SoulsLike/BPIterfaces/BPI_Controller.ToggleHUD`
  (params (bVisible :type Boolean))
  (if bVisible
    (`Widget.SetVisibility` (`self.HUD`) "HitTestInvisible")
    (else
      (`Widget.SetVisibility` (`self.HUD`) "Collapsed"))))

(event `EnhancedInput|/Game/SoulsLike/Input/IA_PauseMenu`
  (params (ActionValue :type Boolean) (ElapsedSeconds :type "Float (double-precision)") (TriggeredSeconds :type "Float (double-precision)") (InputAction :type "InputAction Object Reference" :default "/Game/SoulsLike/Input/IA_PauseMenu.IA_PauseMenu"))
  (:`Started`
    (`GameplayStatics.SetGamePaused` (not (`GameplayStatics.IsGamePaused`)))
    (bind _returnvalue (`|CreateWidget` "/Game/SoulsLike/UI/W_PauseMenu.W_PauseMenu_C"))
    (`UserWidget.AddToViewport` _returnvalue 0)
    (`CommonActivatableWidget.ActivateWidget` _returnvalue)))

(fn `ApplyBuff`
  (params (Effect :type "GameplayEffect Class Reference") (Effect2 :type "GameplayEffect Class Reference"))
  (bind _returnvalue (`AbilitySystemBlueprintLibrary.GetAbilitySystemComponent` (`self.PlayerState`)))
  (`AbilitySystemComponent.BP_ApplyGameplayEffectToSelf` :`self` _returnvalue :`GameplayEffectClass` Effect)
  (`AbilitySystemComponent.BP_ApplyGameplayEffectToSelf` :`self` _returnvalue :`GameplayEffectClass` Effect2))

(fn `ClearEvents`
  (params (Pawn :type "Pawn Object Reference"))
  (remove `PPInventoryComponent.OnSlottedItemChangedDelegateHandle` (`self.BP_InventoryComponent`) (`|CreateDelegate` :!event `UpdateUI`))
  (remove `PPInventoryComponent.OnInventoryItemChangedDelegateHandle` (`self.BP_InventoryComponent`) (`|CreateDelegate` :!event `OnInventoryItemChangedDelegateHandle_Event`)))

(fn `CreateHUD`
  (bind _returnvalue (`|CreateWidget` "/Game/SoulsLike/UI/W_HUD.W_HUD_C" self))
  (bind _output_get (set `self.HUD` _returnvalue))
  (`UserWidget.AddToViewport` _output_get 0))

(fn `HideHUD`
  (`Widget.SetVisibility` (`self.HUD`) "Hidden"))

(fn `OnBuffSelected`
  (params (Buff :type "/Game/SoulsLike/UI/Test/E_BuffTypes Enum" :default "NewEnumerator0"))
  (switch `/Game/SoulsLike/UI/Test/E_BuffTypes` Buff
    (:`NewEnumerator1`
      (`self.ApplyBuff` "/Game/SoulsLike/UI/Test/Effect/GE_BonusHP.GE_BonusHP_C" "/Game/SoulsLike/UI/Test/Effect/GE_RestoreHealth.GE_RestoreHealth_C"))
    (:`NewEnumerator2`
      (`self.ApplyBuff` "/Game/SoulsLike/UI/Test/Effect/GE_BonusMP.GE_BonusMP_C" "/Game/SoulsLike/UI/Test/Effect/GE_RestoreMana.GE_RestoreMana_C"))
    (:`NewEnumerator3`
      (`self.ApplyBuff` "/Game/SoulsLike/UI/Test/Effect/GE_BonusSP.GE_BonusSP_C" "/Game/SoulsLike/UI/Test/Effect/GE_RestoreStamina.GE_RestoreStamina_C")))
  (`GameplayStatics.SetGamePaused` (not (`GameplayStatics.IsGamePaused`))))

(fn `OnLevelUp`
  (`GameplayStatics.SetGamePaused` (not (`GameplayStatics.IsGamePaused`)))
  (bind _returnvalue (`|CreateWidget` "/Game/SoulsLike/UI/Test/W_Buff.W_Buff_C"))
  (`UserWidget.AddToViewport` _returnvalue 0)
  (`CommonActivatableWidget.ActivateWidget` _returnvalue)
  (add `/Game/SoulsLike/UI/Test/W_Buff.OnBuffSelected` _returnvalue (`|CreateDelegate` :!event `OnBuffSelected`))
  (`WidgetBlueprintLibrary.SetInputMode_UIOnlyEx` self _returnvalue))

(fn `SetupEvents`
  (params (Pawn :type "Pawn Object Reference"))
  (add `PPInventoryComponent.OnSlottedItemChangedDelegateHandle` (`self.BP_InventoryComponent`) (`|CreateDelegate` :!event `UpdateUI`))
  (add `PPInventoryComponent.OnInventoryItemChangedDelegateHandle` (`self.BP_InventoryComponent`) (`|CreateDelegate` :!event `OnInventoryItemChangedDelegateHandle_Event`))
  (bind _asppslplayer_state (cast `PPSLPlayerState` (`self.PlayerState`)))
  (add `PPCharacterSet.OnLevelUpDelegate` (`PPSLPlayerState.GetCharacterSet` _asppslplayer_state) (`|CreateDelegate` :!event `OnLevelUp`)))

(fn `ShowHUD`
  (if (`self.bFirstPossess`)
    (`self.CreateHUD`)
    (set `self.bFirstPossess` false)
    (else
      (`Widget.SetVisibility` (`self.HUD`) "HitTestInvisible"))))

(fn `UserConstructionScript`)