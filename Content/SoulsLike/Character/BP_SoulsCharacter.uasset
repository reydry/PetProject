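; Player character for a Souls-like game, built on the Gameplay Ability System.
; Input actions activate, cancel or send events to abilities for rolling, running, attacking, consumables and target lock, with buffered attacks advancing a combo montage index.
; Setup binds the controller's inventory and player-state level-up delegates, applies attribute effects, grants slotted items' abilities and attaches the active weapon.
; Inventory changes refresh abilities and swap hand-socket weapons; death removes both.
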(event `/Game/SoulsLike/BPIterfaces/BPI_Character.SetupPlayer`
  (params (Controller :type "Controller Object Reference"))
  ;[1 1 1] Events
  (`self.SetupEvents` Controller)
  (`self.ApplyEffects`)
  (`self.LoadInventory`))

(event `EnhancedInput|/Game/SoulsLike/Input/IA_ChangeSlot`
  (params (ActionValue :type Boolean) (ElapsedSeconds :type "Float (double-precision)") (TriggeredSeconds :type "Float (double-precision)") (InputAction :type "InputAction Object Reference" :default "/Game/SoulsLike/Input/IA_ChangeSlot.IA_ChangeSlot"))
  ;[1 1 1] Inputs
  (:`Started`
    (`AbilitySystemBlueprintLibrary.SendGameplayEventToActor` self (struct :`TagName` "Ability.Slot.ChangeSlot.Weapon"))))

(event `EnhancedInput|/Game/SoulsLike/Input/IA_Roll`
  (params (ActionValue :type Boolean) (ElapsedSeconds :type "Float (double-precision)") (TriggeredSeconds :type "Float (double-precision)") (InputAction :type "InputAction Object Reference" :default "/Game/SoulsLike/Input/IA_Roll.IA_Roll"))
  ;[1 1 1] Inputs
)

(event `self.ReceiveUnpossessed`
  (params (OldController :type "Controller Object Reference"))
  ;[1 1 1] Events
  (`self.ClearEvents` OldController))

(event `EnhancedInput|/Game/SoulsLike/Input/IA_SwitchTarget`
  (params (ActionValue :type "Float (double-precision)") (ElapsedSeconds :type "Float (double-precision)") (TriggeredSeconds :type "Float (double-precision)") (InputAction :type "InputAction Object Reference" :default "/Game/SoulsLike/Input/IA_SwitchTarget.IA_SwitchTarget"))
  ;[1 1 1] Inputs
  (:`Started`
    (`AbilitySystemBlueprintLibrary.SendGameplayEventToActor` self (struct :`TagName` "Ability.SwitchTarget") (make `GameplayEventData` (struct :`TagName` "Ability.SwitchTarget") null null null null (struct) (struct) (struct) ActionValue))))

(event `EnhancedInput|/Game/SoulsLike/Input/IA_Attack`
  (params (ActionValue :type Boolean) (ElapsedSeconds :type "Float (double-precision)") (TriggeredSeconds :type "Float (double-precision)") (InputAction :type "InputAction Object Reference" :default "/Game/SoulsLike/Input/IA_Attack.IA_Attack"))
  ;[1 1 1] Inputs
)

(event `OnSlottedItemChanged`
  (params (Item :type "PPItem Object Reference") (ItemSlot :type "PPItemSlot Structure"))
  ;[1 1 1] Items
  (`self.RefreshAbilities` Item ItemSlot))

(event `EnhancedInput|/Game/SoulsLike/Input/IA_LockTarget`
  (params (ActionValue :type Boolean) (ElapsedSeconds :type "Float (double-precision)") (TriggeredSeconds :type "Float (double-precision)") (InputAction :type "InputAction Object Reference" :default "/Game/SoulsLike/Input/IA_LockTarget.IA_LockTarget"))
  ;[1 1 1] Inputs
)

(event `EnhancedInput|/Game/SoulsLike/Input/IA_Consumable`
  (params (ActionValue :type Boolean) (ElapsedSeconds :type "Float (double-precision)") (TriggeredSeconds :type "Float (double-precision)") (InputAction :type "InputAction Object Reference" :default "/Game/SoulsLike/Input/IA_Consumable.IA_Consumable"))
  ;[1 1 1] Inputs
)

(event `SaveAttack`
  ;[1 1 1] Combo
  (if (`self.bSaveAttack`)
    (set `self.bSaveAttack` false)))

(event `EnhancedInput|/Game/SoulsLike/Input/IA_Run`
  (params (ActionValue :type Boolean) (ElapsedSeconds :type "Float (double-precision)") (TriggeredSeconds :type "Float (double-precision)") (InputAction :type "InputAction Object Reference" :default "/Game/SoulsLike/Input/IA_Run.IA_Run"))
  ;[1 1 1] Inputs
)

(event `ResetAttack`
  ;[1 1 1] Combo
  (set `self.CurrentMontage` 0)
  (set `self.bSaveAttack` false))

(event `/Game/SoulsLike/BPIterfaces/BPI_Character.Death`
  (`self.DetachWeapon`)
  (`self.RemoveAbilities`))

(fn `ApplyEffects`
  (`AbilitySystemComponent.BP_ApplyGameplayEffectToSelf` :`self` (`AbilitySystemBlueprintLibrary.GetAbilitySystemComponent` null) :`GameplayEffectClass` "/Game/SoulsLike/Stats/GE_PostInitAttributes.GE_PostInitAttributes_C")
  (`AbilitySystemComponent.BP_ApplyGameplayEffectToSelf` :`self` (`AbilitySystemBlueprintLibrary.GetAbilitySystemComponent` null) :`GameplayEffectClass` "/Game/SoulsLike/Stats/GE_StaminaRegeneration.GE_StaminaRegeneration_C")
  (`AbilitySystemComponent.BP_ApplyGameplayEffectToSelf` :`self` (`AbilitySystemBlueprintLibrary.GetAbilitySystemComponent` null) :`GameplayEffectClass` "/Game/SoulsLike/Stats/StatScaling/GE_LevelUp.GE_LevelUp_C")
  (`AbilitySystemComponent.BP_ApplyGameplayEffectToSelf` :`self` (`AbilitySystemBlueprintLibrary.GetAbilitySystemComponent` null) :`GameplayEffectClass` "/Game/SoulsLike/Stats/StatScaling/GE_MaxExpUpdate.GE_MaxExpUpdate_C"))

(fn `AttachWeapon`
  (params (Item :type "PPItem Object Reference"))
  (`/Engine/EditorBlueprintResources/StandardMacros.IsValid` Item
    (:`Is Valid`
      (bind _returnvalue (`|SpawnActorFromClass` (`PPItem.ItemActor` Item) (`self.GetTransform`) "AlwaysSpawn" "MultiplyWithRoot" null self))
      (bind _output_get (set `self.CurrentWeapon` _returnvalue))
      (`self.K2_AttachToComponent` _output_get (`self.Mesh`) "HandSocket" "SnapToTarget" "SnapToTarget" "SnapToTarget" true))))

(fn `ClearEvents`
  (params (Controller :type "Controller Object Reference"))
  (bind _output_get (set `self.InventoryComponent` (`PPInventoryComponent.GetInventoryComponentFromActor` Controller)))
  (remove `PPInventoryComponent.OnSlottedItemChangedDelegateHandle` _output_get (`|CreateDelegate` :!event `OnSlottedItemChanged`))
  (remove `PPInventoryComponent.OnActiveItemChangedDelegateHandle` (`self.InventoryComponent`) (`|CreateDelegate` :!event `Update Item`)))

(fn `DetachWeapon`
  (bind _currentweapon (`self.CurrentWeapon`))
  (`/Engine/EditorBlueprintResources/StandardMacros.IsValid` _currentweapon
    (:`Is Valid`
      (`self.K2_DetachFromActor` _currentweapon "KeepRelative" "KeepRelative" "KeepRelative")
      (`self.K2_DestroyActor` (`self.CurrentWeapon`)))))

(fn `GetCurrentComboMontage`
  (returns (Combo :type Integer))
  (return (`self.CurrentMontage`)))

(fn `GetCurrentWeaponObject`
  (returns (CurrentWeapon :type "PPBaseWeapon Object Reference"))
  (bind _asppbase_weapon (cast `PPBaseWeapon` (`self.CurrentWeapon`)))
  (return _asppbase_weapon))

(fn `GetPPPlayerState`
  (returns (PlayerState :type "/Game/PlayerStates/BP_SLPlayerState Object Reference"))
  (bind _asbp_slplayer_state (cast `/Game/PlayerStates/BP_SLPlayerState` (`self.PlayerState`)))
  (return _asbp_slplayer_state))

(fn `LoadInventory`
  (`/Engine/EditorBlueprintResources/StandardMacros.IsValid` (`self.InventoryComponent`)
    (:`Is Valid`
      (for _array_element (`PPInventoryComponent.GetAllSlottedItems` (`self.InventoryComponent`))
        (`self.GiveAbility` (`PPItem.GrantedAbility` _array_element)))
      (`self.AttachWeapon` (`PPInventoryComponent.GetActiveItemByType` (`self.InventoryComponent`) "Weapon")))))

(fn `OnLevelUp`
  (bind _returnvalue (`AbilitySystemBlueprintLibrary.GetAbilitySystemComponent` null))
  (`AbilitySystemComponent.BP_ApplyGameplayEffectToSelf` :`self` _returnvalue :`GameplayEffectClass` "/Game/SoulsLike/Stats/StatScaling/GE_LevelUp.GE_LevelUp_C")
  (`AbilitySystemComponent.BP_ApplyGameplayEffectToSelf` :`self` _returnvalue :`GameplayEffectClass` "/Game/SoulsLike/Stats/StatScaling/GE_MaxExpUpdate.GE_MaxExpUpdate_C"))

(fn `RefreshAbilities`
  (params (Item :type "PPItem Object Reference") (Slot :type "PPItemSlot Structure"))
  (bind _slot_itemtype (break `PPItemSlot` (`local.Slot`)))
  (`/Engine/EditorBlueprintResources/StandardMacros.IsValid` Item
    (:`Is Valid`
      (`self.GiveAbility` (`PPItem.GrantedAbility` (`local.Item`))))
    (:`Is Not Valid`
      (`self.RemoveAbility` (`self.GetAbility` _slot_itemtype)))))

(fn `SetupEvents`
  (params (Controller :type "Controller Object Reference"))
  (bind _output_get (set `self.InventoryComponent` (`PPInventoryComponent.GetInventoryComponentFromActor` Controller)))
  (add `PPInventoryComponent.OnSlottedItemChangedDelegateHandle` _output_get (`|CreateDelegate` :!event `OnSlottedItemChanged`))
  (add `PPInventoryComponent.OnActiveItemChangedDelegateHandle` (`self.InventoryComponent`) (`|CreateDelegate` :!event `Update Item`))
  (bind _playerstate (`/Game/SoulsLike/BPIterfaces/BPI_Character.GetPPPlayerState`))
  (add `PPCharacterSet.OnLevelUpDelegate` (`PPSLPlayerState.GetCharacterSet` _playerstate) (`|CreateDelegate` :!event `OnLevelUp`)))

(fn `SwitchWeapon`
  (params (Item :type "PPItem Object Reference"))
  (`/Engine/EditorBlueprintResources/StandardMacros.IsValid` Item
    (:`Is Valid`
      (`self.DetachWeapon`)
      (`self.AttachWeapon` (`local.Item`)))
    (:`Is Not Valid`
      (`self.DetachWeapon`))))

(fn `Update Item`
  (params (Item :type "PPItem Object Reference"))
  (switch `EItemType` (`PPItem.ItemType` Item)
    (:`Weapon`
      (`self.SwitchWeapon` (`local.Item`)))))

(fn `UserConstructionScript`)