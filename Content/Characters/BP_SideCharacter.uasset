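; BP_SideCharacter is a player character, apparently side-view, that maps Enhanced Input actions to gameplay abilities for jump, crouch, jump-off and fire.
; Jump, crouch and jump-off activate on press and cancel on release, while fire only activates.
; Reaching the jump apex sets a flag and makes the capsule block a custom trace channel.
; While falling, a short forward trace detects walls, lowering gravity for a post-apex wall slide and restoring it on losing contact.
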(event `self.ReceiveBeginPlay`
  (add `self.OnReachedJumpApex` (delegate `OnReachedJumpApex_Event`)))

(event `OnReachedJumpApex_Event`
  (`PrimitiveComponent.SetCollisionResponseToChannel` (`self.CapsuleComponent`) "ECC_GameTraceChannel1" "ECR_Block")
  (set `self.ApexReached` true))

(event `EnhancedInput|/Game/Input/IA_Jump`
  (params (ActionValue :type Boolean) (ElapsedSeconds :type "Float (double-precision)") (TriggeredSeconds :type "Float (double-precision)") (InputAction :type "InputAction Object Reference" :default "/Game/Input/IA_Jump.IA_Jump"))
  (:`Started`
    (`self.ActivateAbility` "/Game/Abilities/GA_Jump.GA_Jump_C"))
  (:`Completed`
    (`self.CancelAbility` "/Game/Abilities/GA_Jump.GA_Jump_C")))

(event `EnhancedInput|/Game/Input/IA_Crouch`
  (params (ActionValue :type Boolean) (ElapsedSeconds :type "Float (double-precision)") (TriggeredSeconds :type "Float (double-precision)") (InputAction :type "InputAction Object Reference" :default "/Game/Input/IA_Crouch.IA_Crouch"))
  (:`Started`
    (`self.ActivateAbility` "/Game/Abilities/GA_Crouch.GA_Crouch_C"))
  (:`Completed`
    (`self.CancelAbility` "/Game/Abilities/GA_Crouch.GA_Crouch_C")))

(event `EnhancedInput|/Game/Input/IA_JumpOff`
  (params (ActionValue :type Boolean) (ElapsedSeconds :type "Float (double-precision)") (TriggeredSeconds :type "Float (double-precision)") (InputAction :type "InputAction Object Reference" :default "/Game/Input/IA_JumpOff.IA_JumpOff"))
  (:`Started`
    (`self.ActivateAbility` "/Game/Abilities/GA_JumpOff.GA_JumpOff_C"))
  (:`Completed`
    (`self.CancelAbility` "/Game/Abilities/GA_JumpOff.GA_JumpOff_C")))

(event `EnhancedInput|/Game/Input/IA_FIre`
  (params (ActionValue :type Boolean) (ElapsedSeconds :type "Float (double-precision)") (TriggeredSeconds :type "Float (double-precision)") (InputAction :type "InputAction Object Reference" :default "/Game/Input/IA_FIre.IA_FIre"))
  (:`Triggered`
    (`self.ActivateAbility` "/Game/Abilities/GA_Fire.GA_Fire_C")))

(event `self.ReceiveTick`
  (params (DeltaSeconds :type "Float (single-precision)"))
  (if (`NavMovementComponent.IsFalling` (`self.CharacterMovement`))
    (`self.DetectWall`)))

(fn `DetectWall`
  (bind _charactermovement (`self.CharacterMovement`))
  (bind _returnvalue (`self.K2_GetActorLocation` self))
  (bind (_outhit _returnvalue_2) (`KismetSystemLibrary.LineTraceSingleForObjects` :`Start` _returnvalue :`End` (+ _returnvalue (* (`self.GetActorForwardVector` self) 50.0)) :`ObjectTypes` (`|MakeArray` "ObjectTypeQuery1" :!type "EObjectTypeQuery Enum") :`DrawDebugType` "ForOneFrame" :`DrawTime` 1.0))
  (if _returnvalue_2
    (set `self.bTouchingWall` true)
    (if (`self.ApexReached`)
      (set `CharacterMovementComponent.GravityScale` 0.5 _charactermovement))
    (elif (`self.bTouchingWall`)
      (set `self.bTouchingWall` false)
      (set `CharacterMovementComponent.GravityScale` 2.0 _charactermovement))))

(fn `UserConstructionScript`)