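; Gameplay ability for jumping off, which lets the side character pass through whatever uses a custom collision channel, likely drop-through platforms.
; On activation it commits, then sets the avatar capsule's response to GameTraceChannel1 to Ignore, or ends if the commit fails.
; OnEndAbility restores Block; after a successful commit the graph never ends the ability itself, so the ignore lasts until it is ended elsewhere.
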(event `self.K2_ActivateAbility`
  (bind _returnvalue (`self.K2_CommitAbility`))
  (if _returnvalue
    (bind _asbp_side_character (cast `/Game/Characters/BP_SideCharacter` (`self.GetAvatarActorFromActorInfo`)))
    (`PrimitiveComponent.SetCollisionResponseToChannel` (`Character.CapsuleComponent` _asbp_side_character) "ECC_GameTraceChannel1" "ECR_Ignore")
    (else
      (`self.K2_EndAbility`))))

(event `self.K2_OnEndAbility`
  (params (bWasCancelled :type Boolean))
  (bind _asbp_side_character (cast `/Game/Characters/BP_SideCharacter` (`self.GetAvatarActorFromActorInfo`)))
  (`PrimitiveComponent.SetCollisionResponseToChannel` (`Character.CapsuleComponent` _asbp_side_character) "ECC_GameTraceChannel1" "ECR_Block"))