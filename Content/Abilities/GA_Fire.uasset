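; GA_Fire is a Gameplay Ability that fires a BP_Projectile from the avatar along its forward direction.
; On activation it commits the ability, spawns and launches the projectile just ahead of the avatar, then starts a short timer, with FireComplete ending the ability.
; A failed commit ends the ability immediately.
; An unconnected hitscan path remains, using GetTarget's debug-drawn line trace to apply GE_DamageWeapon, but it never runs.
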(event `self.K2_ActivateAbility`
  (bind _returnvalue (`self.GetAvatarActorFromActorInfo`))
  (bind _returnvalue_2 (`self.K2_CommitAbility`))
  (if _returnvalue_2
    (bind _returnvalue_3 (`|SpawnActorFromClass` "/Game/TPSShooter/Weapons/Projectiles/BP_Projectile.BP_Projectile_C" (`KismetMathLibrary.MakeTransform` (+ (`Actor.K2_GetActorLocation` _returnvalue) (* (`Actor.GetActorForwardVector` _returnvalue) 100.0))) "Undefined" "MultiplyWithRoot" null null))
    (`/Engine/EditorBlueprintResources/StandardMacros.IsValid` _returnvalue_3
      (:`Is Valid`
        (`/Game/TPSShooter/Weapons/Projectiles/BP_Projectile.FireInDirection` _returnvalue_3 (`KismetMathLibrary.Conv_RotatorToVector` (`Actor.K2_GetActorRotation` _returnvalue))))
      (:`Is Not Valid`
        _))
    (`KismetSystemLibrary.K2_SetTimerDelegate` (`|CreateDelegate` :!event `FireComplete`) 0.1)
    (else
      (`self.K2_EndAbility`))))

(event `FireComplete`
  (`self.K2_EndAbility`))

(fn `GetTarget`
  (returns (OutTargets :type "GameplayAbilityTargetDataHandle Structure"))
  (bind _returnvalue (`self.GetAvatarActorFromActorInfo`))
  (bind _returnvalue_2 (`Actor.K2_GetActorLocation` _returnvalue))
  (bind _outhit (`KismetSystemLibrary.LineTraceSingle` _returnvalue_2 (+ _returnvalue_2 (* (`Actor.GetActorForwardVector` _returnvalue) 10000.0)) "TraceTypeQuery3" false (`|MakeArray` _returnvalue) "ForDuration"))
  (return (`AbilitySystemBlueprintLibrary.AbilityTargetDataFromHitResult` _outhit)))