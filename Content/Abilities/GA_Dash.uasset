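; GA_Dash is a Gameplay Ability that gives the third-person player a short, fast dash.
; On activation it commits the cost, then applies an additive constant-force root motion that clamps velocity when it finishes.
; GetDirection uses the player's last movement input while moving, or the camera's forward vector when stationary.
; Cooldown is committed only when the dash finishes, just before the ability ends.
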(event `self.K2_ActivateAbility`
  (bind _returnvalue (`self.K2_CommitAbilityCost` true))
  (if _returnvalue
    (`AbilityTask_ApplyRootMotionConstantForce.ApplyRootMotionConstantForce` "None" (`self.GetDirection`) 1850.0 0.25 true null "ClampVelocity" (0.0 0.0 0.0) 1000.0
      (:`OnFinish`
        (`self.K2_CommitAbilityCooldown` false)
        (`self.K2_EndAbility`)))))

(fn `GetDirection`
  (returns (Direction :type "Vector Structure"))
  (bind _asbp_third_person_player (cast `/Game/Characters/BP_ThirdPersonPlayer` (`self.GetAvatarActorFromActorInfo`))
    (:`then`
      (return (select `bool` (`KismetMathLibrary.Vector_IsNearlyZero` (`Actor.GetVelocity` _asbp_third_person_player)) :`false` (`Pawn.GetLastMovementInputVector` _asbp_third_person_player) :`true` (`SceneComponent.GetForwardVector` (`/Game/Characters/BP_ThirdPersonPlayer.Camera` _asbp_third_person_player)))))
    (:`CastFailed`
      (return (0.0 0.0 0.0)))))