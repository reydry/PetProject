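; Gameplay Ability that makes the avatar Character jump, with a wall jump for BP_SideCharacter.
; On successful commit it jumps, enables apex notification, sets the capsule to ignore GameTraceChannel1 and resets ApexReached.
; When touching a wall, it negates the character's yaw and adds a Y/Z launch, using the clamped new yaw for horizontal direction.
; A failed commit ends the ability, and ending calls StopJumping.
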(event `self.K2_ActivateAbility`
  (bind _returnvalue (`self.K2_CommitAbility`))
  (if _returnvalue
    (bind _ascharacter (cast `Character` (`self.GetAvatarActorFromActorInfo`)))
    (`Character.Jump` _ascharacter)
    (set `CharacterMovementComponent.bNotifyApex` true (`Character.CharacterMovement` _ascharacter))
    (`PrimitiveComponent.SetCollisionResponseToChannel` (`Character.CapsuleComponent` _ascharacter) "ECC_GameTraceChannel1" "ECR_Ignore")
    (`self.JumpFromWall` _ascharacter)
    (else
      (`self.K2_EndAbility`))))

(event `self.K2_OnEndAbility`
  (params (bWasCancelled :type Boolean))
  (bind _ascharacter (cast `Character` (`self.GetAvatarActorFromActorInfo`)))
  (`Character.StopJumping` _ascharacter))

(fn `GetLaunchVelocity`
  (returns (Velocity :type "Vector Structure"))
  (bind (_rotation_roll _rotation_pitch _rotation_yaw) (`KismetMathLibrary.BreakRotator` (`self.Rotation`)))
  (return (`KismetMathLibrary.MakeVector` 0.0 (* (`self.y`) (`KismetMathLibrary.FClamp` _rotation_yaw -1.0)) (`self.z`))))

(fn `JumpFromWall`
  (params (Character :type "Character Object Reference"))
  (bind _asbp_side_character (cast `/Game/Characters/BP_SideCharacter` Character))
  (set `/Game/Characters/BP_SideCharacter.ApexReached` false _asbp_side_character)
  (if (`/Game/Characters/BP_SideCharacter.bTouchingWall` _asbp_side_character)
    (bind _newrotation (`self.MakeNewRotation` _asbp_side_character))
    (set `self.Rotation` _newrotation)
    (`Character.LaunchCharacter` _asbp_side_character (`self.GetLaunchVelocity`) false false)
    (`Actor.K2_SetActorRotation` _asbp_side_character (`self.Rotation`) false)))

(fn `MakeNewRotation`
  (params (Character :type "Character Object Reference"))
  (returns (NewRotation :type "Rotator Structure"))
  (bind (_returnvalue_roll _returnvalue_pitch _returnvalue_yaw) (`KismetMathLibrary.BreakRotator` (`Actor.K2_GetActorRotation` Character)))
  (return (`KismetMathLibrary.MakeRotator` _returnvalue_roll _returnvalue_pitch (* _returnvalue_yaw -1.0))))