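; BP_Boss is a boss enemy character that starts its fight when a player enters.
; On entry it plays an entrance montage, turns toward the player and sets them as target on the blackboard and BP_BossAIController.
; Gameplay event listeners drive collision toggles and an AOE sphere trace for pawns at the WeaponTop socket.
; The collision functions, death and player setup are empty stubs, and the trace result is unused.
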(event `self.ReceiveBeginPlay`
  (`AbilityAsync_WaitGameplayEvent.WaitGameplayEventToActor` null (struct :`TagName` "GameplayEvent.Collision.Disable")
    (:`then`
      (`AbilityAsync_WaitGameplayEvent.WaitGameplayEventToActor` null (struct :`TagName` "GameplayEvent.Collision.Enable")
        (:`then`
          (`AbilityAsync_WaitGameplayEvent.WaitGameplayEventToActor` null (struct :`TagName` "GameplayEvent.TraceObjects.AOE")
            (:`EventReceived`
              (`self.TraceAOE`))))
        (:`EventReceived`
          (`self.CollisionEnable`))))
    (:`EventReceived`
      (`self.CollisionDisable`))))

(event `/Game/SoulsLike/BPIterfaces/BPI_Character.Death`)

(event `/Game/SoulsLike/BPIterfaces/BPI_Character.SetupPlayer`
  (params (Controller :type "Controller Object Reference")))

(event `OnPlayerEntered`
  (params (Player :type "PPCharacter Object Reference"))
  (bind _returnvalue (`AIBlueprintHelperLibrary.GetAIController` self))
  (`self.PlayAnimMontage` "/Game/BossyEnemy/Animations/RootMotion/AM_Boss_BattleEntrance_RM.AM_Boss_BattleEntrance_RM")
  (`BlackboardComponent.SetValueAsObject` (`AIBlueprintHelperLibrary.GetBlackboard` _returnvalue) "Target" Player)
  (`self.K2_SetActorRotation` (`KismetMathLibrary.FindLookAtRotation` (`self.K2_GetActorLocation`) (`self.K2_GetActorLocation` Player)))
  (bind _asbp_boss_aicontroller (cast `/Game/BossyEnemy/Controller/BP_BossAIController` _returnvalue))
  (set `/Game/BossyEnemy/Controller/BP_BossAIController.Target` Player _asbp_boss_aicontroller))

(fn `CollisionDisable`)

(fn `CollisionEnable`)

(fn `GetCurrentComboMontage`
  (returns (Combo :type Integer))
  (return 0))

(fn `GetCurrentWeaponObject`
  (returns (CurrentWeapon :type "PPBaseWeapon Object Reference"))
  (return null))

(fn `GetPPPlayerState`
  (returns (PlayerState :type "/Game/PlayerStates/BP_SLPlayerState Object Reference")))

(fn `TraceAOE`
  (bind _returnvalue (`SceneComponent.GetSocketLocation` (`self.Mesh`) "WeaponTop"))
  (`KismetSystemLibrary.SphereTraceSingleForObjects` _returnvalue _returnvalue 100.0 (`|MakeArray` "ObjectTypeQuery3" :!type "EObjectTypeQuery Enum") false (`|MakeArray` self :!type "Actor Object Reference") "ForDuration"))

(fn `UserConstructionScript`)