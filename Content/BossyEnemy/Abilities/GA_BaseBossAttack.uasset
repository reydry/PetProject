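; Base gameplay ability for boss attacks that plays an attack montage and reacts to gameplay events during it.
; On activation it commits, plays the configured montage, and starts a wait for each tag in its event tag container, routing received events to EventReceived.
; EventReceived is empty here, and the ability ends when the montage completes, blends out, is interrupted or cancelled, or when commit fails.
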(event `self.K2_ActivateAbility`
  (bind _returnvalue (`self.K2_CommitAbility`))
  (if _returnvalue
    (`AbilityTask_PlayMontageAndWait.CreatePlayMontageAndWaitProxy` "None" (`self.Montage`) (`self.Rate`)
      (:`then`
        (for _array_element (`BlueprintGameplayTagLibrary.BreakGameplayTagContainer` (`self.EventTagContainer`))
          (bind (_asynctaskproxy _payload) (`AbilityTask_WaitGameplayEvent.WaitGameplayEvent` _array_element null)
            (:`EventReceived`
              (`self.EventReceived` _payload)))))
      (:`OnCompleted`
        (`self.K2_EndAbility` :!label _label))
      (:`OnBlendOut`
        (goto _label))
      (:`OnInterrupted`
        (goto _label))
      (:`OnCancelled`
        (goto _label)))
    (else
      (`self.K2_EndAbility`))))

(event `self.K2_OnEndAbility`
  (params (bWasCancelled :type Boolean))
  (`KismetSystemLibrary.PrintString` "ended")
  (`self.OnAbilityEnd`))

(fn `EventReceived`
  (params (Payload :type "GameplayEventData Structure")))