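; BP_Projectile is a weapon projectile for the TPS shooter that deals damage through the Gameplay Ability System.
; FireInDirection launches it by setting the projectile movement velocity to the direction times the initial speed.
; Its sphere overlap ignores BP_ThirdPersonPlayer and destroys the projectile on any other actor.
; Targets with an Ability System Component first receive GE_DamageWeapon, applied by their own component to itself.
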(event `self.Sphere.OnComponentBeginOverlap`
  (params (OverlappedComponent :type "PrimitiveComponent Object Reference") (OtherActor :type "Actor Object Reference") (OtherComp :type "PrimitiveComponent Object Reference") (OtherBodyIndex :type Integer) (bFromSweep :type Boolean) (SweepResult :type "HitResult Structure (by ref)"))
  (bind _returnvalue (`AbilitySystemBlueprintLibrary.GetAbilitySystemComponent` OtherActor))
  (cast `/Game/Characters/BP_ThirdPersonPlayer` OtherActor
    (:`CastFailed`
      (`/Engine/EditorBlueprintResources/StandardMacros.IsValid` _returnvalue
        (:`Is Valid`
          (`AbilitySystemComponent.BP_ApplyGameplayEffectToTarget` :`self` _returnvalue :`GameplayEffectClass` "/Game/GameplayEffects/GE_DamageWeapon.GE_DamageWeapon_C" :`Target` _returnvalue)
          (`self.K2_DestroyActor`))
        (:`Is Not Valid`
          (`self.K2_DestroyActor`))))))

(fn `FireInDirection`
  (params (Direction :type "Vector Structure"))
  (set `MovementComponent.Velocity` (* Direction (`ProjectileMovementComponent.InitialSpeed` (`self.ProjectileMovement`))) (`self.ProjectileMovement`)))

(fn `UserConstructionScript`)