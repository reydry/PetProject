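; Gameplay ability for firing the rocket launcher in the TPS shooter, currently implementing only the recoil push on the player.
; On activation it prints a debug string and applies a short root motion constant force opposite the camera's forward vector, keeping the last root motion velocity afterward.
; The direction comes from the third-person player avatar's camera, or a zero vector if the cast fails.
; It spawns no projectile and never commits or ends the ability itself.
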(event `self.K2_ActivateAbility`
  (`parent.K2_ActivateAbility`)
  (`KismetSystemLibrary.PrintString` "GA_RocketlauncherFire")
  (`AbilityTask_ApplyRootMotionConstantForce.ApplyRootMotionConstantForce` "None" (* (`self.GetDirection`) -1.0) 500.0 0.1 false null "MaintainLastRootMotionVelocity"))

(fn `GetDirection`
  (returns (Direction :type "Vector Structure"))
  (bind _asbp_third_person_player (cast `/Game/Characters/BP_ThirdPersonPlayer` (`self.GetAvatarActorFromActorInfo`))
    (:`then`
      (return (`SceneComponent.GetForwardVector` (`/Game/Characters/BP_ThirdPersonPlayer.Camera` _asbp_third_person_player))))
    (:`CastFailed`
      (return (0.0 0.0 0.0)))))